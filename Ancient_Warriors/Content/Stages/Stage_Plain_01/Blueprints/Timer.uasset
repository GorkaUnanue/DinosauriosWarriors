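; Reusable count-up timer Blueprint in the Stage_Plain_01 stage folder, advanced by its caller through Update rather than Tick.
; Update adds delta time up to TotalTime and returns a finished flag plus normalized progress, also exposed by GetLerpingTime.
; SetNewTime changes the duration and leaves the timer completed until Reset zeroes it.
; GetCurrentTime returns raw time, but its Finished uses strict greater-than, unlike Update.
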(event EventBeginPlay)

(event EventTick
  (params (DeltaSeconds :type Float%20%28single-precision%29)))

(fn Update
  (params (Dt :type Float%20%28single-precision%29))
  (bind _totaltime (Variables|Default|GetTotalTime))
  (if (>= (Variables|Default|GetmTimer) _totaltime)
    _
    (else
      (Variables|Default|SetmTimer (Math|Float|Clamp(Float) (+ Dt (Variables|Default|GetmTimer)) 0.0 (Variables|Default|GetTotalTime)))))
  (return (>= (Variables|Default|GetmTimer) _totaltime) (/ (Variables|Default|GetmTimer) _totaltime)))

(fn GetCurrentTime
  (bind _mtimer (Variables|Default|GetmTimer))
  (return _mtimer (> _mtimer (Variables|Default|GetTotalTime))))

(fn SetNewTime
  (params (NewTime :type Float%20%28single-precision%29))
  (bind _output_get (Variables|Default|SetTotalTime NewTime))
  (Variables|Default|SetmTimer _output_get))

(fn Reset
  (Variables|Default|SetmTimer 0.0))

(fn GetLerpingTime
  (return (/ (Variables|Default|GetmTimer) (Variables|Default|GetTotalTime))))