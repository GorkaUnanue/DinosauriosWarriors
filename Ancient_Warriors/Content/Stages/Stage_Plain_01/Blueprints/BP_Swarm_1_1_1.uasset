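; BP_Swarm_1_1_1 is a swarm actor for stage Plain 01 that spawns two Olkathu enemies at fixed transforms on BeginPlay.
; A helper spawns each AI_Enemy and initializes its skin, color and entry animation, randomized except the first one's skin and color.
; It stores them in an array and keeps an enemy count, printed every tick.
; EnemyMinus1 decrements that count but is not called here, and death-check fragments are unwired.
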(event EventBeginPlay
  (Variables|Default|SetOlkathu_Skin 0)
  (Variables|Default|SetOlkathu_Color 0)
  (Variables|Default|SetOlkathu_Entry_Animation (Math|Random|RandomIntegerinRange 0 2))
  (bind _olkathu_enemy (CallFunction|CreateOlkathuEnemy (Math|Transform|MakeTransform "1929.660034,-265.239868,95.998726" "0,180.000000, 0")))
  (bind _output_get (Variables|Default|SetOlkathu_1 _olkathu_enemy))
  (Utilities|Array|Add (Variables|Default|GetA_Enemy) _output_get)
  (Variables|Default|SetOlkathu_Skin (Math|Random|RandomIntegerinRange 0 2))
  (Variables|Default|SetOlkathu_Color (Math|Random|RandomIntegerinRange 0 2))
  (Variables|Default|SetOlkathu_Entry_Animation (Math|Random|RandomIntegerinRange 0 2))
  (bind _olkathu_enemy_2 (CallFunction|CreateOlkathuEnemy (Math|Transform|MakeTransform "1729.660034,177.443771,95.998726" "0,180.000000, 0")))
  (bind _output_get_2 (Variables|Default|SetOlkathu_2 _olkathu_enemy_2))
  (Utilities|Array|Add (Variables|Default|GetA_Enemy) _output_get_2)
  (Variables|Default|SetEnemy_Number 2))

(event Collision|EventActorBeginOverlap
  (params (OtherActor :type Actor%20Object%20Reference)))

(event EventTick
  (params (DeltaSeconds :type Float%20%28single-precision%29))
  (Development|PrintString (Utilities|String|ToString(Integer) (Variables|Default|GetEnemy_Number))))

(fn ConstructionScript)

(fn CreateOlkathuEnemy
  (params (SpawnTransform :type Transform))
  (bind _returnvalue (Game|SpawnActorfromClass "/Game/Characters/Enemies/AI_Enemy.AI_Enemy_C" SpawnTransform "Undefined" 0 0))
  (Default|Initialize _returnvalue (Variables|Default|GetOlkathu_Skin) (Variables|Default|GetOlkathu_Color) (Variables|Default|GetOlkathu_Entry_Animation))
  (return 0))

(fn EnemyMinus1
  (Variables|Default|SetEnemy_Number (+ (Variables|Default|GetEnemy_Number) -1)))