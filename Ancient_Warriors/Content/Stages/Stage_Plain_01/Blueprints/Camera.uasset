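; Stage camera actor that switches between settings-driven modes: static, follow, directional follow, player-to-point, cylindrical and spline-path variants.
; Each Tick resolves the mode's position and rotation, optionally clamps XY, and interpolates the actor toward it.
; ChangeCameraValues queues new settings, defaulting the target to Camera_Offset, and starts timers.
; During transitions it evaluates both modes and sine-eases between them, while spring arm length eases separately on its own timer.
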(event Custom|ChangeCameraValues
  (params (NewSettings :type Camera%20Settings%20Structure))
  (CallFunction|SetNewCameraSettings NewSettings))

(event EventBeginPlay
  (CallFunction|SetInitialState))

(event Collision|EventActorBeginOverlap
  (params (OtherActor :type Actor%20Object%20Reference)))

(event EventTick
  (params (DeltaSeconds :type Float%20%28single-precision%29))
  (CallFunction|UpdateCamera DeltaSeconds)
  (CallFunction|UpdateSpringArm DeltaSeconds))

(fn ConstructionScript)

(fn SetInitialState
  (bind _springarm (Variables|Default|GetSpringArm))
  (bind _outactors (Actor|GetAllActorsOfClass "/Game/Stages/Stage_Plain_01/Blueprints/Camera_Offset.Camera_Offset_C"))
  (for _array_element _outactors
    (bind _structout (Utilities|Struct|SetmembersinCameraSettings (Variables|Default|GetCurrentSettings) (Transformation|GetWorldLocation _springarm) (Variables|/Script/Engine.SpringArmComponent|GetTargetArmLength _springarm) (Class|SpringArmComponent|GetTargetRotation _springarm)))
    (bind _output_get (Variables|Default|SetCurrentSettings _structout))
    (switch Utilities|FlowControl|Switch|SwitchonCameraTypes (.mCameraType (Utilities|Struct|BreakCameraSettings (Variables|Default|GetCurrentSettings)))
      (:NewEnumerator1
        (bind _structout_2 (Utilities|Struct|SetmembersinCameraSettings _output_get (Transformation|GetActorLocation _array_element)))
        (Variables|Default|SetCurrentSettings _structout_2)))))

(fn UpdateCamera
  (params (Dt :type Float%20%28single-precision%29))
  (bind _currentsettings (Variables|Default|GetCurrentSettings))
  (bind _nextsettings (Variables|Default|GetNextSettings))
  (bind _currentsettings_2 (Variables|Default|GetCurrentSettings))
  (if (Variables|Default|GetNeedToChange)
    (bind (_new_position _new_rotator) (CallFunction|UpdateSettingCamera _currentsettings))
    (bind _finaltransform (CallFunction|SmoothMovement _new_position _new_rotator Dt _currentsettings))
    (bind (_new_position_2 _new_rotator_2) (CallFunction|UpdateSettingCamera _nextsettings))
    (bind _finaltransform_2 (CallFunction|SmoothMovement _new_position_2 _new_rotator_2 Dt _nextsettings))
    (bind _finaltransform_3 (CallFunction|LerpStates Dt _finaltransform _finaltransform_2))
    (Transformation|SetActorTransform _finaltransform_3)
    (else
      (bind (_new_position_3 _new_rotator_3) (CallFunction|UpdateSettingCamera _currentsettings_2))
      (bind _finaltransform_4 (CallFunction|SmoothMovement _new_position_3 _new_rotator_3 Dt _currentsettings_2))
      (Transformation|SetActorTransform _finaltransform_4))))

(fn UpdateSettingCamera
  (params (NewParam :type Camera%20Settings%20Structure))
  (switch Utilities|FlowControl|Switch|SwitchonCameraTypes (.mCameraType (Utilities|Struct|BreakCameraSettings NewParam))
    (:NewEnumerator0
      ;[1 1 1] Switch of the camera type
      (bind (_new_position _new_rotator) (CallFunction|UpdateStaticCamera))
      (return _new_position _new_rotator))
    (:NewEnumerator1
      (bind (_new_position_2 _new_rotator_2) (CallFunction|UpdateFollowCamera))
      (return _new_position_2 _new_rotator_2))
    (:NewEnumerator2
      (bind (_new_position_3 _new_rotator_3) (CallFunction|UpdateMoveBetweenTargetandPos))
      (return _new_position_3 _new_rotator_3))
    (:NewEnumerator3
      (bind (_new_position_4 _new_rotator_4) (CallFunction|UpdatePathFocusCamera))
      (return _new_position_4 _new_rotator_4))
    (:NewEnumerator4
      (bind (_new_position_5 _new_rotator_5) (CallFunction|UpdateCylinderCamera))
      (return _new_position_5 _new_rotator_5))
    (:NewEnumerator5
      (bind (_new_position_6 _new_rotator_6) (CallFunction|UpdatePathWithoutRotationCamera))
      (return _new_position_6 _new_rotator_6))
    (:NewEnumerator6
      (bind (_new_position_7 _new_rotator_7) (CallFunction|UpdateFollowinDirectionCamera))
      (return _new_position_7 _new_rotator_7))
    (:NewEnumerator7
      (bind (_new_position_8 _new_rotator_8) (CallFunction|UpdatePathFocusPlayerPathCamera))
      (return _new_position_8 _new_rotator_8))))

(fn UpdateStaticCamera
  (params (NewParam :type Camera%20Settings%20Structure))
  (bind (_mcameratype _mchangetime _newposition _springarmdistance _cameraorientation) (Utilities|Struct|BreakCameraSettings NewParam))
  (return _newposition _cameraorientation))

(fn UpdateFollowCamera
  (params (NewParam :type Camera%20Settings%20Structure))
  (bind (_mcameratype _mchangetime _newposition _springarmdistance _cameraorientation _target) (Utilities|Struct|BreakCameraSettings NewParam))
  (return (Transformation|GetActorLocation _target) _cameraorientation))

(fn UpdateMoveBetweenTargetandPos
  (params (NewParam :type Camera%20Settings%20Structure))
  (bind (_newposition _springarmdistance _cameraorientation _target _camerapath _offsetdistance) (Utilities|Struct|BreakCameraSettings NewParam))
  (return (+ _newposition (* (* (- (Transformation|GetActorLocation _target) _newposition) "1.000000,1.000000, 0") _offsetdistance)) _cameraorientation))

(fn UpdatePathFocusCamera
  (params (NewParam :type Camera%20Settings%20Structure))
  (bind (_target _camerapath) (Utilities|Struct|BreakCameraSettings NewParam))
  (bind _pointincamerasplinebasedinplayerpath (CallFunction|GetCameraLocationonPath _target _camerapath))
  (return _pointincamerasplinebasedinplayerpath (Math|Rotator|FindLookatRotation _pointincamerasplinebasedinplayerpath (Transformation|GetActorLocation _target))))

(fn GetCameraLocationonPath
  (params (Player :type Actor%20Object%20Reference) (Path :type Camera%20Path%20Object%20Reference))
  (bind _returnvalue (Transformation|GetActorLocation Player))
  (bind _cameraspline (Variables|/Game/Stages/Stage_Plain_01/Blueprints/CameraPath.CameraPath_C|GetCameraSpline Path))
  (bind _playerspline (Variables|/Game/Stages/Stage_Plain_01/Blueprints/CameraPath.CameraPath_C|GetPlayerSpline Path))
  (bind _returnvalue_2 (Class|SplineComponent|FindInputKeyClosesttoWorldLocation _playerspline _returnvalue))
  (return (Class|SplineComponent|GetLocationatSplineInputKey _cameraspline (* (Math|Conversions|ToFloat(Integer) (Spline|GetNumberOfSplinePoints _cameraspline)) (/ _returnvalue_2 (Math|Conversions|ToFloat(Integer) (Spline|GetNumberOfSplinePoints _playerspline)))) "Local") (Class|SplineComponent|GetLocationatSplineInputKey _playerspline _returnvalue_2 "Local") (Class|SplineComponent|GetLocationatSplineInputKey _cameraspline (Class|SplineComponent|FindInputKeyClosesttoWorldLocation _cameraspline _returnvalue) "Local")))

(fn UpdateCylinderCamera
  (params (NewParam :type Camera%20Settings%20Structure))
  (bind (_newposition _target) (Utilities|Struct|BreakCameraSettings NewParam))
  (bind (_x _y _z) (Math|Vector|BreakVector _newposition))
  (bind _returnvalue (Transformation|GetActorLocation _target))
  (return (Math|Vector|MakeVector _x _y (+ _z (.Z (Math|Vector|BreakVector _returnvalue)))) (Math|Rotator|FindLookatRotation _newposition _returnvalue)))

(fn UpdatePathWithoutRotationCamera
  (params (NewParam :type Camera%20Settings%20Structure))
  (bind (_cameraorientation _target _camerapath) (Utilities|Struct|BreakCameraSettings NewParam))
  (bind _pointincameraspline (CallFunction|GetCameraLocationonPath _target _camerapath))
  (return _pointincameraspline _cameraorientation))

(fn UpdateFollowinDirectionCamera
  (params (NewParam :type Camera%20Settings%20Structure))
  (bind (_newposition _cameraorientation _target _direction) (Utilities|Struct|BreakCameraSettings NewParam))
  (return (+ _newposition (Math|Vector|ProjectVectorontoVector (- (Class|KismetMathLibrary|ProjectPointontoPlane (Transformation|GetActorLocation _target) _newposition (Math|Vector|Normalize (Math|Vector|CrossProduct (Math|Vector|GetForwardVector _cameraorientation) _direction))) _newposition) _direction)) _cameraorientation))

(fn UpdatePathFocusPlayerPathCamera
  (params (NewParam :type Camera%20Settings%20Structure))
  (bind (_target _camerapath) (Utilities|Struct|BreakCameraSettings NewParam))
  (bind (_pointincamerasplinebasedinplayerpath _pointinplayerspline) (CallFunction|GetCameraLocationonPath _target _camerapath))
  (return _pointincamerasplinebasedinplayerpath (Math|Rotator|FindLookatRotation _pointincamerasplinebasedinplayerpath _pointinplayerspline)))

(fn SmoothMovement
  (params (Target_Location :type Vector) (Target_Rotation :type Rotator) (DeltaTime :type Float%20%28single-precision%29) (CameraSetting :type Camera%20Settings%20Structure))
  (bind (_camerapath _useminmax _minpos _maxpos) (Utilities|Struct|BreakCameraSettings CameraSetting))
  (bind (_x _y _z) (Math|Vector|BreakVector Target_Location))
  (bind (_x_2 _y_2) (Math|Vector|BreakVector _minpos))
  (bind (_x_3 _y_3) (Math|Vector|BreakVector _maxpos))
  (if _useminmax
    (LocalVariables|SetLocationToSet (Math|Vector|MakeVector (Math|Float|Clamp(Float) _x _x_2 _x_3) (Math|Float|Clamp(Float) _y _y_2 _y_3) _z))
    (else
      (LocalVariables|SetLocationToSet Target_Location)))
  (return (Class|KismetMathLibrary|TInterpto (Transformation|GetActorTransform) (Math|Transform|MakeTransform (LocalVariables|GetLocationToSet) Target_Rotation "1,1,1") DeltaTime 0.0)))

(fn LerpStates
  (params (Dt :type Float%20%28single-precision%29) (Transform0 :type Transform) (Transform1 :type Transform))
  (bind (_finished _currenttime) (Default|Update (Variables|Default|GetmTimer) Dt))
  (bind _output_get (Variables|Default|SetNeedToChange (not _finished)))
  (if _output_get
    _
    (else
      (Variables|Default|SetCurrentSettings (Variables|Default|GetNextSettings))
      (Variables|Default|SetNextSettings (Utilities|Struct|MakeCameraSettings 0 -5))))
  (return (Math|Interpolation|Ease "SinusoidalInOut" _currenttime Transform0 Transform1)))

(fn UpdateSpringArm
  (params (Dt :type Float%20%28single-precision%29))
  (bind _lerp_time (Default|GetLerpingTime (Variables|Default|GetmTimer)))
  (if (> _lerp_time 0.5)
    (bind _springarm (CallFunction|LerpSpringArm Dt))
    (Variables|/Script/Engine.SpringArmComponent|SetTargetArmLength (Variables|Default|GetSpringArm) _springarm)))

(fn LerpSpringArm
  (params (Dt :type Float%20%28single-precision%29))
  (bind _currenttime (Default|Update (Variables|Default|GetSpringArmTimer) Dt))
  (return (Math|Interpolation|Ease "EaseInOut" _currenttime (Variables|Default|GetCurrentArm) (Variables|Default|GetNextArm) 2.0)))

(fn SetNewCameraSettings
  (params (NextSettings :type Camera%20Settings%20Structure))
  (bind (_mchangetime _target _camerapath _id) (Utilities|Struct|BreakCameraSettings NextSettings))
  (if (not (== (.Id (Utilities|Struct|BreakCameraSettings (Variables|Default|GetNextSettings))) _id))
    (if (or (and (Variables|Default|GetNeedToChange) (== (.Id (Utilities|Struct|BreakCameraSettings (Variables|Default|GetCurrentSettings))) _id)) (== (.Id (Utilities|Struct|BreakCameraSettings (Variables|Default|GetCurrentSettings))) _id))
      (Variables|Default|SetCurrentSettings (Utilities|Struct|MakeCameraSettings "NewEnumerator1" (Transformation|GetActorLocation) (Variables|/Script/Engine.SpringArmComponent|GetTargetArmLength (Variables|Default|GetSpringArm)) (Transformation|GetActorRotation))))
    (Utilities|IsValid _target
      (:Is%20Valid
        (Variables|Default|SetNextSettings NextSettings)
        (Variables|Default|SetNeedToChange true :!label _label)
        (Default|SetNewTime (Variables|Default|GetmTimer) _mchangetime)
        (Default|SetNewTime (Variables|Default|GetSpringArmTimer) _mchangetime)
        (Variables|Default|SetCurrentArm (.SpringArmDistance (Utilities|Struct|BreakCameraSettings (Variables|Default|GetCurrentSettings))))
        (Variables|Default|SetNextArm (.mChangeTime (Utilities|Struct|BreakCameraSettings (Variables|Default|GetNextSettings)))))
      (:Is%20Not%20Valid
        (bind _outactors (Actor|GetAllActorsOfClass "/Game/Stages/Stage_Plain_01/Blueprints/Camera_Offset.Camera_Offset_C"))
        (for _array_element _outactors
          (bind _structout (Utilities|Struct|SetmembersinCameraSettings NextSettings _array_element))
          (Variables|Default|SetNextSettings _structout)
          (goto _label))))))