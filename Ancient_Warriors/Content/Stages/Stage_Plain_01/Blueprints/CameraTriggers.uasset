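; Camera trigger volume that switches the stage camera's settings when the CatawCharacter overlaps it.
; On BeginPlay it bakes its SpringArm transform and length, Arrow direction and its index among all triggers into a settings struct, optionally targeting the player pawn.
; The SpringArm is then destroyed, serving only as a placement guide.
; On overlap it sends the struct to every Camera actor and the offset distance to the character.
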(event EventBeginPlay
  (bind _springarm (Variables|Default|GetSpringArm))
  (bind _outactors (Actor|GetAllActorsOfClass "CameraTriggers_C"))
  (for (_array_element _array_index) _outactors
    (if (== _array_element self)
      (bind _structout (Utilities|Struct|SetmembersinCameraSettings (Variables|Default|GetmCameraSettings) (Transformation|GetWorldLocation _springarm) (Variables|/Script/Engine.SpringArmComponent|GetTargetArmLength _springarm) (Transformation|GetWorldRotation _springarm) _array_index (Math|Vector|GetForwardVector (Variables|Default|GetArrow))))
      (if (Variables|Default|GetPlayerAsTarget)
        (bind _structout_2 (Utilities|Struct|SetmembersinCameraSettings _structout (Game|Player|GetPlayerPawn 0)))
        (Variables|Default|SetmCameraSettings _structout_2)
        (else
          (Variables|Default|SetmCameraSettings _structout)))
      (Components|DestroyComponent (Variables|Default|GetSpringArm)))))

(event Collision|EventActorBeginOverlap
  (params (OtherActor :type Actor%20Object%20Reference))
  (bind _mcamerasettings (Variables|Default|GetmCameraSettings))
  (bind _ascataw_character (Utilities|Casting|CastToCatawCharacter OtherActor))
  (bind _outactors (Actor|GetAllActorsOfClass "/Game/Stages/Stage_Plain_01/Blueprints/Camera.Camera_C"))
  (for _array_element _outactors
    (Default|ChangeCameraValues _array_element _mcamerasettings)
    (Default|ChangeCameraOffset _ascataw_character (.OffsetDistance (Utilities|Struct|BreakCameraSettings _mcamerasettings)))))

(event EventTick
  (params (DeltaSeconds :type Float%20%28single-precision%29)))

(fn ConstructionScript)