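; Main menu actor that highlights the selected New Game, Load Game or Options item by making its lettering glow.
; On BeginPlay it creates dynamic materials for the three item meshes and binds to the CatawMainMenu player character's selection dispatcher.
; Each dispatch reads that character's MainMenuOption, raises Emissive on the matching item and zeroes the others, with debug prints.
; Leftover option-cycling and level-opening logic is disconnected and never runs.
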(event Custom|SelectMainModeUp
  (bind _output_get (Variables|Default|SetMainMenuOption (Variables|/Game/ThirdPersonBP/Blueprints/CatawMainMenu.CatawMainMenu_C|GetMainMenuOption (stale EventBeginPlay _ascataw_main_menu))))
  (Development|PrintString (Utilities|String|ToString(Integer) _output_get))
  (if (== (Variables|Default|GetMainMenuOption) 1)
    (Development|PrintString (Utilities|String|ToString(Integer) (Variables|Default|GetMainMenuOption)))
    (Rendering|Material|SetScalarParameterValue (stale EventBeginPlay _returnvalue) "Emissive" 5e+01 :!class /Script/Engine.MaterialInstanceDynamic)
    (Rendering|Material|SetScalarParameterValue (stale EventBeginPlay _returnvalue_2) "Emissive" 0.0 :!class /Script/Engine.MaterialInstanceDynamic)
    (Rendering|Material|SetScalarParameterValue (stale EventBeginPlay _returnvalue_3) "Emissive" 0.0 :!class /Script/Engine.MaterialInstanceDynamic)
    (elif (== (Variables|Default|GetMainMenuOption) 2)
      (Development|PrintString (Utilities|String|ToString(Integer) (Variables|Default|GetMainMenuOption)))
      (Rendering|Material|SetScalarParameterValue (stale EventBeginPlay _returnvalue) "Emissive" 0.0 :!class /Script/Engine.MaterialInstanceDynamic)
      (Rendering|Material|SetScalarParameterValue (stale EventBeginPlay _returnvalue_2) "Emissive" 5e+01 :!class /Script/Engine.MaterialInstanceDynamic)
      (Rendering|Material|SetScalarParameterValue (stale EventBeginPlay _returnvalue_3) "Emissive" 0.0 :!class /Script/Engine.MaterialInstanceDynamic)
      (elif (== (Variables|Default|GetMainMenuOption) 3)
        (Development|PrintString (Utilities|String|ToString(Integer) (Variables|Default|GetMainMenuOption)))
        (Rendering|Material|SetScalarParameterValue (stale EventBeginPlay _returnvalue) "Emissive" 0.0 :!class /Script/Engine.MaterialInstanceDynamic)
        (Rendering|Material|SetScalarParameterValue (stale EventBeginPlay _returnvalue_2) "Emissive" 0.0 :!class /Script/Engine.MaterialInstanceDynamic)
        (Rendering|Material|SetScalarParameterValue (stale EventBeginPlay _returnvalue_3) "Emissive" 5e+01 :!class /Script/Engine.MaterialInstanceDynamic)))))

(event EventBeginPlay
  (bind _ascataw_main_menu (Utilities|Casting|CastToCatawMainMenu (Game|GetPlayerCharacter 0)))
  (EventDispatchers|BindEventtoSelectMainModeEventDispatcher _ascataw_main_menu (delegate Custom|SelectMainModeUp))
  (bind _returnvalue (Rendering|Material|CreateDynamicMaterialInstance (Variables|Default|GetMainMenuNewGame_Item) 1 "/Game/Stages/Main_Menu/Assets/Menu_Item_Letters_New_Game.Menu_Item_Letters_New_Game" "None" :!class /Script/Engine.PrimitiveComponent))
  (bind _returnvalue_2 (Rendering|Material|CreateDynamicMaterialInstance (Variables|Default|GetMainMenuLoadGame_Item) 1 "/Game/Stages/Main_Menu/Assets/Menu_Item_Letters_Load_Game.Menu_Item_Letters_Load_Game" "None" :!class /Script/Engine.PrimitiveComponent))
  (bind _returnvalue_3 (Rendering|Material|CreateDynamicMaterialInstance (Variables|Default|GetMainMenuOptions_Item) 1 "/Game/Stages/Main_Menu/Assets/Menu_Item_Letters_Options.Menu_Item_Letters_Options" "None" :!class /Script/Engine.PrimitiveComponent))
  (Input|EnableInput (Game|GetPlayerController 0)))

(event Collision|EventActorBeginOverlap
  (params (OtherActor :type Actor%20Object%20Reference)))

(event EventTick
  (params (DeltaSeconds :type Float%20%28single-precision%29)))

(event Input|KeyboardEvents|S
  (params (Key :type Key%20Structure)))

(event Input|KeyboardEvents|W
  (params (Key :type Key%20Structure)))

(event Input|GamepadEvents|GamepadLeftStickUp
  (params (Key :type Key%20Structure)))

(event Input|GamepadEvents|GamepadLeftStickDown
  (params (Key :type Key%20Structure)))

(fn ConstructionScript)